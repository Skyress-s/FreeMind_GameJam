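; ScarySpikes is a spike hazard Blueprint that damages the player character and exists at different positions in two dimensions.
; A hit on its Cube component casts to MyMainCharacterBP, calls Damage and launches the character upward.
; Every Tick reads the player pawn's InsanityDimenson flag and snaps the actor, without sweep, to DimensionBlend's TwoDSpace location when true or ThreeDSpace when false.
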(event OnComponentHit(Cube)
  (params (HitComponent :type Primitive%20Component%20Object%20Reference) (OtherActor :type Actor%20Object%20Reference) (OtherComp :type Primitive%20Component%20Object%20Reference) (NormalImpulse :type Vector :default "0, 0, 0") (Hit :type Hit%20Result%20Structure%20%28by%20ref%29))
  (bind _asmy_main_character_bp (Utilities|Casting|CastToMyMainCharacterBP OtherActor))
  (Class|MainCharacter|Damage _asmy_main_character_bp)
  (Character|LaunchCharacter _asmy_main_character_bp "0, 0,500.000000" false false))

(event EventBeginPlay)

(event Collision|EventActorBeginOverlap
  (params (OtherActor :type Actor%20Object%20Reference)))

(event EventTick
  (params (DeltaSeconds :type Float%20%28single-precision%29))
  (bind _dimensionblend (Variables|Default|GetDimensionBlend))
  (bind _asmy_main_character_bp (Utilities|Casting|CastToMyMainCharacterBP (Game|Player|GetPlayerPawn 0)))
  (if (Variables|/Script/FreeMind.MainCharacter|GetbInsanityDimenson _asmy_main_character_bp)
    (Transformation|SetActorLocation (Variables|/Script/FreeMind.DimensionBlendComponent|GetTwoDSpace _dimensionblend) false false)
    (else
      (Transformation|SetActorLocation (Variables|/Script/FreeMind.DimensionBlendComponent|GetThreeDSpace _dimensionblend) false false))))

(fn ConstructionScript)